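; Actor that watches the level for the end-game condition and tells the player character when it is reached.
; Each Tick it gathers all BP_Rat, BP_Blahaj and BP_Froggy actors with GetAllActorsOfClass.
; Once none of the three classes remain, it sets a one-shot flag and calls EndGame on the player's BPC_FirstPersonCharacter.
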(event EventBeginPlay)

(event Collision|EventActorBeginOverlap
  (params (OtherActor :type Actor%20Object%20Reference)))

(event EventTick
  (params (DeltaSeconds :type Float%20%28single-precision%29))
  (if (not (Variables|Default|GetTriggeredEndGame))
    (bind _outactors (Actor|GetAllActorsOfClass "/Game/Blueprints/Interactable/WandInteract/BP_Rat.BP_Rat_C"))
    (Variables|Default|SetRat _outactors)
    (bind _outactors_2 (Actor|GetAllActorsOfClass "/Game/Blueprints/Interactable/BP_Blahaj.BP_Blahaj_C"))
    (Variables|Default|SetBlahaj _outactors_2)
    (bind _outactors_3 (Actor|GetAllActorsOfClass "/Game/Blueprints/Interactable/BP_Froggy.BP_Froggy_C"))
    (Variables|Default|SetFroggy _outactors_3)
    (if (Math|Boolean|ANDBoolean (Utilities|Array|IsEmpty (Variables|Default|GetRat)) (Utilities|Array|IsEmpty (Variables|Default|GetBlahaj)) (Utilities|Array|IsEmpty (Variables|Default|GetFroggy)))
      (Variables|Default|SetTriggeredEndGame true)
      (bind _asbpc_first_person_character (Utilities|Casting|CastToBPC_FirstPersonCharacter (Game|GetPlayerCharacter 0)))
      (Default|EndGame _asbpc_first_person_character))))

(fn ConstructionScript)